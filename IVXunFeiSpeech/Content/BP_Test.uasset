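; Test Blueprint that exercises the XunFei (iFlytek) speech plugin: Chinese streaming and real-time speech-to-text, text-to-speech and translation.
; Streaming recognition binds and unbinds init, response, completed and error delegates on the XunFei TTS subsystem through separate setup and exit events.
; Real-time recognition and translation pass callbacks directly to their start calls.
; Callbacks print status or results to screen, while synthesized speech plays as 2D sound.
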(event Custom|初始化语音识别
  (bind _returnvalue (|IVXunFeiTTSSubsystem))
  (EventDispatchers|AssignStreamingSTTInitdDelegate _returnvalue (delegate Custom|语音识别初始化完成的回调))
  (EventDispatchers|AssignStreamingSTTResponseDelegate _returnvalue (delegate Custom|语音识别反馈的回调))
  (EventDispatchers|AssignStreamingSTTCompletedDelegate _returnvalue (delegate Custom|语音识别完成的回调))
  (EventDispatchers|AssignStreamingSTTErrorDelegate _returnvalue (delegate Custom|语音识别出错的回调)))

(event Custom|CustomEvent_0
  (params (OutSrcText :type String))
  (Development|PrintString (Utilities|String|Append "实时语音识别没有翻译的结果：" OutSrcText)))

(event Custom|开始流式语音识别
  (Class|IVXunFeiSpeechFunctionLibrary|XunFeiBeginStreamingSpeechtoText (Utilities|Struct|MakeXunFeiStreamingSTTOptions "zh_cn" "iat")))

(event Custom|停止流式语音识别
  (Class|IVXunFeiSpeechFunctionLibrary|XunFeiStopStreamingSpeechtoText))

(event Custom|CustomEvent
  (params (bInitResult :type Boolean) (InitRespMessage :type String))
  (Development|PrintString "初始化实时语音识别"))

(event Custom|开始语音合成
  (params (InText :type String) (TTSOptions :type Xun%20Fei%20TTS%20Options%20Structure))
  (bind _soundwave (|XunFeiTexttoSoundWave InText TTSOptions)
    (:then
      (Audio|PlaySound2D _soundwave 1.0 1.0 0.0 0 0))))

(event Custom|开始翻译
  (params (SourceText :type String) (XunFeiTranslateOptions :type Xun%20Fei%20Translate%20Options%20Structure))
  (Class|IVXunFeiSpeechFunctionLibrary|XunFeiBeginTranslate SourceText XunFeiTranslateOptions (delegate Custom|翻译结果的回调)))

(event Custom|停止翻译
  (Class|IVXunFeiSpeechFunctionLibrary|XunFeiStopTranslate))

(event Custom|翻译结果的回调
  (params (FinalResult :type String))
  (Development|PrintString FinalResult))

(event Custom|退出语音识别
  (bind _returnvalue (|IVXunFeiTTSSubsystem))
  (EventDispatchers|UnbindallEventsfromStreamingSTTInitdDelegate _returnvalue)
  (EventDispatchers|UnbindallEventsfromStreamingSTTResponseDelegate _returnvalue)
  (EventDispatchers|UnbindallEventsfromStreamingSTTCompletedDelegate _returnvalue)
  (EventDispatchers|UnbindallEventsfromStreamingSTTErrorDelegate _returnvalue))

(event Custom|语音识别初始化完成的回调
  (Development|PrintString "[语音识别]：初始化完成"))

(event Custom|停止实时语音识别（一般用流式）
  (Class|IVXunFeiSpeechFunctionLibrary|XunFeiStopRealTimeSpeechtoText))

(event Custom|语音识别反馈的回调
  (params (OutResult :type String))
  (Development|PrintString (Utilities|String|Append "[语音识别]：反馈 ： " OutResult)))

(event Custom|语音识别完成的回调
  (params (FinalResult :type String))
  (Development|PrintString (Utilities|String|Append "[语音识别]：最终的结果：" FinalResult)))

(event Custom|语音识别出错的回调
  (params (ErrorMessage :type String))
  (Development|PrintString (Utilities|String|Append "[语音识别]：出错：" ErrorMessage)))

(event Custom|CustomEvent_1
  (params (OutSrcText :type String) (OutDstText :type String))
  (Development|PrintString (Utilities|String|Append "实时语音识别没有翻译的结果：" OutSrcText "实时语音识别有翻译的结果：" OutDstText)))

(event Custom|开始实时语音识别（一般用流式）
  (Class|IVXunFeiSpeechFunctionLibrary|XunFeiBeginRealTimeSpeechtoText (Utilities|Struct|MakeXunFeiRealTimeSTTOptions "cn" false) (delegate Custom|CustomEvent) (delegate Custom|CustomEvent_0) (delegate Custom|CustomEvent_1)))

(fn ConstructionScript)