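; BP_TestVoicePlayer is a test Blueprint that wraps a VoicePlayerComponent, exposing voice playback controls and printing a debug log for most actions.
; Init and exit events bind and unbind the component's started, task-started and completed delegates.
; Queue events start, stop, enqueue text-plus-SoundWave tasks, permit completion once empty, and set volume.
; Separate functions play one-off voices with completion delegates, from a SoundWave or a WAV converted from the project's Resources/Wav folder.
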(event Custom|退出语音播放
  (bind _voiceplayercomponent (Variables|Default|GetVoicePlayerComponent))
  (EventDispatchers|UnbindallEventsfromVoicePlayerStartedDelegate _voiceplayercomponent)
  (EventDispatchers|UnbindallEventsfromTaskStartedDelegate _voiceplayercomponent)
  (EventDispatchers|UnbindallEventsfromVoicePlayerCompletedDelegate _voiceplayercomponent))

(event Custom|设置语音播放的音量
  (params (NewVolumeMultiplier :type Float%20%28single-precision%29))
  (Audio|Components|Audio|SetVolumeMultiplier (Variables|Default|GetVoicePlayerComponent) NewVolumeMultiplier :!class /Script/Engine.AudioComponent))

(event Custom|一个语音开始播放的回调
  (params (SourceText :type String) (Duration :type Float%20%28single-precision%29))
  (Development|PrintString (Utilities|String|Append "[语音播放]：播放内容为：" SourceText)))

(event Custom|开始语音播放
  (Development|PrintString "[语音播放]：开始")
  (Class|VoicePlayerComponent|StartVoicePlayer (Variables|Default|GetVoicePlayerComponent)))

(event Custom|语音播放初始化完成的回调
  (Development|PrintString "[语音播放]：初始化完成"))

(event Custom|初始化语音播放
  (bind _voiceplayercomponent (Variables|Default|GetVoicePlayerComponent))
  (EventDispatchers|BindEventtoVoicePlayerStartedDelegate _voiceplayercomponent (delegate Custom|语音播放初始化完成的回调))
  (EventDispatchers|AssignTaskStartedDelegate _voiceplayercomponent (delegate Custom|一个语音开始播放的回调))
  (EventDispatchers|BindEventtoVoicePlayerCompletedDelegate _voiceplayercomponent (delegate Custom|语音播放结束的回调)))

(event Custom|语音播放结束的回调
  (Development|PrintString "[语音播放]：结束"))

(event Custom|添加语音播放任务
  (params (SourceContent :type String) (SoundWave :type Sound%20Wave%20Object%20Reference%20%28by%20ref%29))
  (Development|PrintString (Utilities|String|Append "[语音播放]：添加语音播放任务文本为：" SourceContent))
  (Class|VoicePlayerComponent|EnqueueTasktoQueue (Variables|Default|GetVoicePlayerComponent) SourceContent SoundWave))

(event Custom|停止语音播放
  (Development|PrintString "[语音播放]：停止")
  (Class|VoicePlayerComponent|StopVoicePlayer (Variables|Default|GetVoicePlayerComponent)))

(event Custom|当所有语音播放任务完成时可以停止队列工作
  (Development|PrintString "[语音播放]：可以停止工作")
  (Class|VoicePlayerComponent|CanQueueCompletedWhileQueueEmpty (Variables|Default|GetVoicePlayerComponent)))

(fn ConstructionScript)

(fn 播放单独的语音文件
  (params (FileName :type String) (InCompletedDelegate :type Delegate))
  (Development|PrintString (Utilities|String|Append "[独立语音播放]：播放语音文件为：" FileName))
  (bind _returnvalue (Class|IVisualFileHeplerBPLibrary|ConvertWavFiletoSoundWave (Utilities|String|Append (Class|KismetSystemLibrary|GetProjectDirectory) "Resources/Wav") FileName))
  (Class|VoicePlayerComponent|PlayVoiceOnce (Variables|Default|GetVoicePlayerComponent) _returnvalue InCompletedDelegate))

(fn 播放单独的语音
  (params (InSoundWave :type Sound%20Wave%20Object%20Reference) (InPlayVoiceOnceCompletedDelegate :type Delegate))
  (Development|PrintString (Utilities|String|Append "[独立语音播放]：播放语音为：" (Utilities|GetDisplayName InSoundWave)))
  (Class|VoicePlayerComponent|PlayVoiceOnce (Variables|Default|GetVoicePlayerComponent) InSoundWave InPlayVoiceOnceCompletedDelegate))