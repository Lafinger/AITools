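; Voice-to-image controller that turns spoken Chinese into ComfyUI text-to-image jobs and shows the results in an SD widget.
; A wake word cancels current work and starts XunFei streaming recognition; the result is translated to English and submitted as the prompt.
; The widget's generate button also submits prompts.
; A separate TTS queue feeds a voice player queue, using DoOnce to start playback on the first finished clip.
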(event Custom|终止语音交互
  (Development|PrintString "[全局]：终止语音交互")
  (CallFunction|停止语音唤醒)
  (CallFunction|停止语音交互))

(event Custom|停止语音交互
  (Development|PrintString "[全局]：停止语音交互")
  (CallFunction|停止语音识别)
  (CallFunction|停止语音合成)
  (CallFunction|停止语音播放))

(event Custom|合成语音文件
  (params (Vcn :type String) (SourceText :type String) (FilePath :type String))
  (if (and (not (Utilities|Array|IsEmpty SourceText)) (not (Utilities|Array|IsEmpty FilePath)))
    (|XunFeiTexttoWavFile SourceText (Utilities|Struct|MakeXunFeiTTSOptions Vcn 50) FilePath
      (:OnConnectionError
        (Development|PrintString (Utilities|String|ToString(Text) (Utilities|Text|FormatText "[工具]：合成语音文件{0}Error，文本为：{1}！" FilePath SourceText))))
      (:OnClose
        (Development|PrintString (Utilities|String|ToString(Text) (Utilities|Text|FormatText "[工具]：合成语音文件{0}完成，文本为：{1}" FilePath SourceText)))))
    (else
      (Development|PrintString "[工具]：需要合成的文本或路径为空 Error!"))))

(event Custom|初始化语音交互
  (Utilities|FlowControl|Sequence
    (:then_0
      (CallFunction|初始化语音唤醒))
    (:then_1
      (CallFunction|初始化语音识别))
    (:then_2
      (CallFunction|初始化语音合成))
    (:then_3
      (CallFunction|初始化语音播放))))

(event Custom|退出语音交互
  (if true
    (CallFunction|终止语音交互)
    (Utilities|FlowControl|Sequence
      (:then_0
        (CallFunction|退出语音合成))
      (:then_1
        (CallFunction|退出语音播放))
      (:then_2
        (CallFunction|退出语音识别))
      (:then_3
        (CallFunction|退出语音唤醒)))))

(event Custom|播放语料库
  (params (Question :type String) (Answer :type String))
  (Variables|Default|SetTempQuestion Question)
  (CallFunction|添加语音合成任务 Answer true)
  (CallFunction|开始语音合成)
  (CallFunction|当所有语音合成任务完成时可以停止队列工作))

(event Custom|语音唤醒触发的回调
  (Development|PrintString "[语音唤醒]：触发")
  (CallFunction|停止音声图)
  (CallFunction|开始语音识别 (Utilities|Struct|MakeXunFeiStreamingSTTOptions "zh_cn" "iat")))

(event Custom|语音唤醒完成的回调
  (Development|PrintString "[语音唤醒]：完成"))

(event Custom|语音唤醒出错的回调
  (params (ErrorCode :type Integer))
  (Development|PrintString (Utilities|String|Append "[语音唤醒]：出错， 错误码：" (Utilities|String|ToString(Integer) ErrorCode)))
  (CallFunction|播放单独的语音文件))

(event Custom|停止语音唤醒
  (Development|PrintString "[语音唤醒]：停止")
  (Class|VoiceWakeUpSubsystem|Stop (|VoiceWakeUpSubsystem)))

(event Custom|开始语音唤醒
  (Development|PrintString "[语音唤醒]：开始")
  (Class|VoiceWakeUpSubsystem|Start (|VoiceWakeUpSubsystem)))

(event Custom|退出语音唤醒
  (bind _returnvalue (|VoiceWakeUpSubsystem))
  (Class|VoiceWakeUpSubsystem|Stop _returnvalue)
  (Class|VoiceWakeUpSubsystem|MsgLogout _returnvalue)
  (EventDispatchers|UnbindallEventsfromWakeUpTriggerDelegate _returnvalue)
  (EventDispatchers|UnbindallEventsfromWakeUpCompletedDelegate _returnvalue)
  (EventDispatchers|UnbindallEventsfromWakeUpFailedDelegate _returnvalue))

(event Custom|初始化语音唤醒
  (bind _returnvalue (|VoiceWakeUpSubsystem))
  (bind _returnvalue_2 (Class|VoiceWakeUpSubsystem|MsgLogin _returnvalue))
  (if _returnvalue_2
    (EventDispatchers|BindEventtoWakeUpTriggerDelegate _returnvalue (delegate Custom|语音唤醒触发的回调))
    (EventDispatchers|BindEventtoWakeUpCompletedDelegate _returnvalue (delegate Custom|语音唤醒完成的回调))
    (EventDispatchers|BindEventtoWakeUpFailedDelegate _returnvalue (delegate Custom|语音唤醒出错的回调))
    (else
      (Development|PrintString "[语音唤醒]：登录失败"))))

(event Custom|初始化语音识别
  (bind _returnvalue (|IVXunFeiTTSSubsystem))
  (EventDispatchers|AssignStreamingSTTInitdDelegate _returnvalue (delegate Custom|语音识别初始化完成的回调))
  (EventDispatchers|AssignStreamingSTTResponseDelegate _returnvalue (delegate Custom|语音识别反馈的回调))
  (EventDispatchers|AssignStreamingSTTCompletedDelegate _returnvalue (delegate Custom|语音识别完成的回调))
  (EventDispatchers|AssignStreamingSTTErrorDelegate _returnvalue (delegate Custom|语音识别出错的回调)))

(event Custom|停止语音识别
  (Development|PrintString "[语音识别]：停止")
  (Class|IVXunFeiSpeechFunctionLibrary|XunFeiStopStreamingSpeechtoText))

(event Custom|退出语音识别
  (bind _returnvalue (|IVXunFeiTTSSubsystem))
  (EventDispatchers|UnbindallEventsfromStreamingSTTInitdDelegate _returnvalue)
  (EventDispatchers|UnbindallEventsfromStreamingSTTResponseDelegate _returnvalue)
  (EventDispatchers|UnbindallEventsfromStreamingSTTCompletedDelegate _returnvalue)
  (EventDispatchers|UnbindallEventsfromStreamingSTTErrorDelegate _returnvalue))

(event Custom|语音识别初始化完成的回调
  (Development|PrintString "[语音识别]：初始化完成"))

(event Custom|开始语音识别
  (params (XunFeiStreamingSTTOptions :type Xun%20Fei%20Streaming%20STT%20Options%20Structure))
  (Development|PrintString "[语音识别]：开始")
  (Class|IVXunFeiSpeechFunctionLibrary|XunFeiBeginStreamingSpeechtoText XunFeiStreamingSTTOptions))

(event Custom|语音识别反馈的回调
  (params (OutResult :type String))
  (Development|PrintString (Utilities|String|Append "[语音识别]：反馈 ： " OutResult)))

(event Custom|语音识别完成的回调
  (params (FinalResult :type String))
  (Development|PrintString (Utilities|String|Append "[语音识别]：最终的结果：" FinalResult))
  (if (Utilities|Array|IsEmpty FinalResult)
    (CallFunction|语音识别出错的回调 "识别为空")
    (else
      (CallFunction|开始语音唤醒)
      (bind _output_get (Variables|Default|SetTempQuestion FinalResult))
      (Class|IVXunFeiSpeechFunctionLibrary|XunFeiBeginTranslate _output_get (Utilities|Struct|MakeXunFeiTranslateOptions 3 "" "cn" "en") (delegate Custom|语音识别后翻译的回调)))))

(event Custom|语音识别出错的回调
  (params (ErrorMessage :type String))
  (Development|PrintString (Utilities|String|Append "[语音识别]：出错：" ErrorMessage))
  (CallFunction|开始语音唤醒)
  (CallFunction|播放单独的语音文件))

(event Custom|语音识别后翻译的回调
  (params (bIsSuccess :type Boolean) (FinalResult :type String))
  (if bIsSuccess
    (Default|提交文生图任务 (Variables|Default|GetComfyUIManager) FinalResult)
    (Default|SetPromptText (Variables|Default|GetSDWidget) FinalResult)
    (else
      (CallFunction|语音识别出错的回调 FinalResult))))

(event Custom|初始化语音合成
  (bind _returnvalue (|VoiceSynthesisSubsystem))
  (EventDispatchers|BindEventtoQueueWorkingStartDelegate _returnvalue (delegate Custom|语音合成初始化完成的回调))
  (EventDispatchers|BindEventtoTaskCompletedDelegate _returnvalue (delegate Custom|语音合成一个完成的回调))
  (EventDispatchers|BindEventtoQueueWorkingCompletedDelegate _returnvalue (delegate Custom|语音合成所有任务完成的回调))
  (EventDispatchers|BindEventtoTaskErrorDelegate _returnvalue (delegate Custom|语音合成一个出错的回调)))

(event Custom|退出语音合成
  (bind _returnvalue (|VoiceSynthesisSubsystem))
  (EventDispatchers|UnbindallEventsfromQueueWorkingStartDelegate _returnvalue)
  (EventDispatchers|UnbindallEventsfromTaskCompletedDelegate _returnvalue)
  (EventDispatchers|UnbindallEventsfromQueueWorkingCompletedDelegate _returnvalue)
  (EventDispatchers|UnbindallEventsfromTaskErrorDelegate _returnvalue))

(event Custom|语音合成所有任务完成的回调
  (Development|PrintString "[语音合成]：所有语音合成结束")
  (CallFunction|当所有语音播放任务完成时可以停止队列工作))

(event Custom|语音合成初始化完成的回调
  (Development|PrintString "[语音合成]：初始化完成")
  (Utilities|FlowControl|Sequence
    (:then_1
      (Utilities|FlowControl|DoOnce false) ; enters at Reset
    )))

(event Custom|语音合成一个完成的回调
  (params (VoiceText :type String) (SourceText :type String) (FileAbsolutePath :type String) (SoundWave :type Sound%20Wave%20Object%20Reference))
  (Utilities|IsValid SoundWave
    (:Is%20Valid
      (Development|PrintString (Utilities|String|Append "[语音合成]：成功，合成内容为：" VoiceText))
      (CallFunction|添加语音播放任务 SourceText SoundWave)
      (Utilities|FlowControl|DoOnce false
        (:Completed
          (CallFunction|开始语音播放))))))

(event Custom|语音合成一个出错的回调
  (params (ErrorMessage :type String))
  (Development|PrintString (Utilities|String|Append "[语音合成]：出错：" ErrorMessage))
  (CallFunction|播放单独的语音文件))

(event Custom|开始语音合成
  (Development|PrintString "[语音合成]：开始")
  (Class|VoiceSynthesisSubsystem|StartQueueWorking (|VoiceSynthesisSubsystem) false))

(event Custom|添加语音合成任务
  (params (InText :type String) (IsQA :type Boolean))
  (Development|PrintString (Utilities|String|Append "[语音合成]：添加语音合成任务文本为：" InText))
  (bind (_voicetext _uitext) (CallFunction|处理合成语音与UI显示文本 InText))
  (Class|VoiceSynthesisSubsystem|EnqueueVoiceSynthesisTask (|VoiceSynthesisSubsystem) _voicetext _uitext (Utilities|Struct|MakeXunFeiTTSOptions "x4_mengmengneutral" 50)))

(event Custom|停止语音合成
  (Development|PrintString "[语音合成]：停止")
  (Class|IVXunFeiSpeechFunctionLibrary|XunFeiStopTranslate)
  (Class|VoiceSynthesisSubsystem|StopQueueWorking (|VoiceSynthesisSubsystem)))

(event Custom|当所有语音合成任务完成时可以停止队列工作
  (Development|PrintString "[语音合成]：可以停止工作")
  (Class|VoiceSynthesisSubsystem|CanQueueCompletedWhileQueueEmpty (|VoiceSynthesisSubsystem)))

(event Custom|退出语音播放
  (bind _voiceplayercomponent (Variables|Default|GetVoicePlayerComponent))
  (EventDispatchers|UnbindallEventsfromVoicePlayerStartedDelegate _voiceplayercomponent)
  (EventDispatchers|UnbindallEventsfromTaskStartedDelegate _voiceplayercomponent)
  (EventDispatchers|UnbindallEventsfromVoicePlayerCompletedDelegate _voiceplayercomponent))

(event Custom|设置语音播放的音量
  (params (NewVolumeMultiplier :type Float%20%28single-precision%29))
  (Class|VoicePlayerComponent|SetVoicePlayerVolume (Variables|Default|GetVoicePlayerComponent) NewVolumeMultiplier)
  (Development|PrintString (Utilities|String|Append "[系统设置]：当前音量为：" (Utilities|String|ToString(Float) NewVolumeMultiplier))))

(event Custom|一个语音开始播放的回调
  (params (SourceText :type String) (Duration :type Float%20%28single-precision%29))
  (Development|PrintString (Utilities|String|Append "[语音播放]：播放内容为：" SourceText)))

(event Custom|减小音量
  (bind _voicevolumemultiplier (Variables|Default|GetVoiceVolumeMultiplier))
  (if (> _voicevolumemultiplier 1.0)
    (bind _result (Math|Float|DecrementFloat _voicevolumemultiplier)
      (:%20%20
        (CallFunction|设置语音播放的音量 _result)))))

(event Custom|开始语音播放
  (Development|PrintString "[语音播放]：开始")
  (Class|VoicePlayerComponent|StartVoicePlayer (Variables|Default|GetVoicePlayerComponent)))

(event Custom|语音播放初始化完成的回调
  (Development|PrintString "[语音播放]：初始化完成"))

(event Custom|初始化语音播放
  (bind _voiceplayercomponent (Variables|Default|GetVoicePlayerComponent))
  (EventDispatchers|BindEventtoVoicePlayerStartedDelegate _voiceplayercomponent (delegate Custom|语音播放初始化完成的回调))
  (EventDispatchers|BindEventtoTaskStartedDelegate _voiceplayercomponent (delegate Custom|一个语音开始播放的回调))
  (EventDispatchers|BindEventtoVoicePlayerCompletedDelegate _voiceplayercomponent (delegate Custom|语音播放结束的回调)))

(event Custom|语音播放结束的回调
  (Development|PrintString "[语音播放]：结束"))

(event Custom|增大音量
  (bind _voicevolumemultiplier (Variables|Default|GetVoiceVolumeMultiplier))
  (if (< _voicevolumemultiplier 1e+01)
    (bind _result (Math|Float|IncrementFloat _voicevolumemultiplier)
      (:%20%20
        (CallFunction|设置语音播放的音量 _result)))))

(event Custom|添加语音播放任务
  (params (SourceContent :type String) (SoundWave :type Sound%20Wave%20Object%20Reference%20%28by%20ref%29))
  (Development|PrintString (Utilities|String|Append "[语音播放]：添加语音播放任务文本为：" SourceContent))
  (Class|VoicePlayerComponent|EnqueueTasktoQueue (Variables|Default|GetVoicePlayerComponent) SourceContent SoundWave))

(event Custom|停止语音播放
  (Development|PrintString "[语音播放]：停止")
  (Class|VoicePlayerComponent|StopVoicePlayer (Variables|Default|GetVoicePlayerComponent)))

(event Custom|当所有语音播放任务完成时可以停止队列工作
  (Development|PrintString "[语音播放]：可以停止工作")
  (Class|VoicePlayerComponent|CanQueueCompletedWhileQueueEmpty (Variables|Default|GetVoicePlayerComponent)))

(event Custom|初始化音生图
  (bind _returnvalue (Game|GetPlayerController 0))
  (bind _comfyuimanager (Variables|Default|GetComfyUIManager))
  (Utilities|FlowControl|Sequence
    (:then_0
      (CallFunction|初始化语音交互))
    (:then_1
      (Utilities|FlowControl|Sequence
        (:then_0
          (bind _returnvalue_2 (UserInterface|CreateWidget "/StableDiffusionServices/WBP_SDExample.WBP_SDExample_C" _returnvalue))
          (bind _output_get (Variables|Default|SetSDWidget _returnvalue_2))
          (UserInterface|Viewport|AddtoViewport _output_get 0)
          (Variables|/Script/Engine.PlayerController|SetbShowMouseCursor _returnvalue true))
        (:then_1
          (EventDispatchers|BindEventtoTTIImageGeneratedDispatcher _comfyuimanager (delegate Custom|文生图生成完成的回调))
          (Default|开启全局监听触发事件 _comfyuimanager))
        (:then_2
          (EventDispatchers|BindEventtoGenerateBtnClickDispatcher (Variables|Default|GetSDWidget) (delegate Custom|点击图片生成按钮触发的回调)))))))

(event Custom|退出音生图
  (bind _comfyuimanager (Variables|Default|GetComfyUIManager))
  (Utilities|FlowControl|Sequence
    (:then_0
      (CallFunction|退出语音交互))
    (:then_1
      (Default|停止文生图任务 _comfyuimanager)
      (Default|停止监听事件 _comfyuimanager))))

(event Custom|停止音声图
  (Utilities|FlowControl|Sequence
    (:then_0
      (CallFunction|停止语音交互))
    (:then_1
      (Default|停止文生图任务 (Variables|Default|GetComfyUIManager)))))

(event Custom|文生图生成完成的回调
  (params (Texture2DDynamic :type Texture%202D%20Dynamic%20Object%20Reference))
  (Default|ShowComfyUISDImage (Variables|Default|GetSDWidget) Texture2DDynamic))

(event Custom|点击图片生成按钮触发的回调
  (Default|提交文生图任务 (Variables|Default|GetComfyUIManager) (Default|GetPromptText (Variables|Default|GetSDWidget))))

(fn ConstructionScript)

(fn 播放单独的语音文件
  (params (FileName :type String) (InCompletedDelegate :type Delegate))
  (Development|PrintString (Utilities|String|Append "[独立语音播放]：播放语音文件为：" FileName))
  (CallFunction|停止语音交互)
  (bind _returnvalue (Class|IVisualFileHeplerBPLibrary|ConvertWavFiletoSoundWave FileName FileName))
  (Class|VoicePlayerComponent|PlayVoiceOnce (Variables|Default|GetVoicePlayerComponent) _returnvalue InCompletedDelegate))

(fn 处理合成语音与UI显示文本
  (params (InText :type String))
  (return InText InText))