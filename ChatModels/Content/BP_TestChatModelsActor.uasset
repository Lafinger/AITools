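; Test actor that wraps a chat model component for a voice large-language-model feature and logs its lifecycle to screen.
; Init and exit events bind and unbind the component's start, generated, completed and error delegates.
; Start passes a question and model type to the component and stop halts it.
; Callbacks print initialization, each generated sentence chunk, completion and error reasons.
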(event Custom|停止大模型
  (Development|PrintString "[语音大模型]：停止")
  (Default|StopChatModel (Variables|Default|GetBP_ChatModelComponent)))

(event Custom|初始化大模型
  (bind _bp_chatmodelcomponent (Variables|Default|GetBP_ChatModelComponent))
  (EventDispatchers|BindEventtoChatModelStartDelegate _bp_chatmodelcomponent (delegate Custom|大模型初始化完成的回调))
  (EventDispatchers|BindEventtoChatModelGeneratedDelegate _bp_chatmodelcomponent (delegate Custom|大模型分句生成的回调))
  (EventDispatchers|BindEventtoChatModelCompletedDelegate _bp_chatmodelcomponent (delegate Custom|大模型输出完成的回调))
  (EventDispatchers|BindEventtoChatModelErrorDelegate _bp_chatmodelcomponent (delegate Custom|大模型输出出错的回调)))

(event Custom|大模型输出出错的回调
  (params (Reason :type String))
  (Development|PrintString (Utilities|String|Append "[语音大模型]：出错：" Reason)))

(event Custom|退出大模型
  (bind _bp_chatmodelcomponent (Variables|Default|GetBP_ChatModelComponent))
  (EventDispatchers|UnbindallEventsfromChatModelStartDelegate _bp_chatmodelcomponent)
  (EventDispatchers|UnbindallEventsfromChatModelGeneratedDelegate _bp_chatmodelcomponent)
  (EventDispatchers|UnbindallEventsfromChatModelCompletedDelegate _bp_chatmodelcomponent)
  (EventDispatchers|UnbindallEventsfromChatModelErrorDelegate _bp_chatmodelcomponent))

(event Custom|开始大模型
  (params (Question :type String) (ChatModelType :type EDifyModelType%20Enum :default "Spark"))
  (Development|PrintString "[语音大模型]：开始")
  (Default|StartChatModel (Variables|Default|GetBP_ChatModelComponent) Question ChatModelType))

(event Custom|大模型初始化完成的回调
  (Development|PrintString "[语音大模型]：初始化完成"))

(event Custom|大模型分句生成的回调
  (params (Generated :type String))
  (Development|PrintString (Utilities|String|Append "[语音大模型]：生成的分句为：" Generated)))

(event Custom|大模型输出完成的回调
  (Development|PrintString "[语音大模型]：结束"))

(fn ConstructionScript)