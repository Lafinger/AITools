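; Chat model component that streams answers to a question from a Dify-style LLM service, apparently for voice synthesis.
; An async HTTP request returns server-sent events, whose answer fields are joined and diffed against the last response to get new text.
; Accumulated text is broadcast through delegates in punctuation-delimited chunks.
; On completion it flushes the remainder, splitting long text at Chinese full stops, and signals completion.
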(event Custom|StartChatModel
  (params (Question :type String) (ChatModelType :type EDifyModelType%20Enum :default "Spark"))
  (if (Variables|Default|GetIsRuning)
    (CallFunction|OnChatModelError "[语音大模型]：已经在运行")
    (else
      (Variables|Default|SetIsRuning true)
      (CallFunction|ClearCache)
      (bind _output_get (Variables|Default|SetTempQuestion Question))
      (bind _output_get_2 (Variables|Default|SetTempType ChatModelType))
      (Development|PrintString (Utilities|String|Append "[语音大模型]：输入的问题：{" _output_get "}" "选择的类型：{" (Utilities|String|EnumtoString _output_get_2) "}"))
      (Default|CallChatModelStartDelegate)
      (bind (_asynctaskproxy _message) (|AsyncHttpRequest (Variables|Default|GetConversationID) _output_get "POST" _output_get_2 false)
        (:then
          (bind _output_get_3 (Variables|Default|SetRequest%20Task _asynctaskproxy))
          (Utilities|IsValid _output_get_3
            (:Is%20Not%20Valid
              (CallFunction|OnChatModelError "[大模型]：输出或配置有问题"))))
        (:ResponseDelegate
          (Variables|Default|SetTemp "")
          (for _array_element (Utilities|String|ParseIntoArray (Utilities|String|Replace _message "event: ping") "data:")
            (if (not (Utilities|String|Contains _array_element " ping"))
              (Variables|Default|SetConversationID (Class|IVJsonObject|GetStringField (Class|IVJsonLibrary|ConvStringtoJsonObject _array_element) "conversation_id"))
              (Variables|Default|SetTemp (Utilities|String|Append (Variables|Default|GetTemp) (Class|IVJsonObject|GetStringField (Class|IVJsonLibrary|ConvStringtoJsonObject _array_element) "answer")))))
          (bind _returnvalue (Class|ChatModelsSubsystem|RemoveStringLineBreak (Subsystems|GetChatModelsSubsystem) (Variables|Default|GetTemp)))
          (if (.ReturnValue (Utilities|String|Split _returnvalue (Variables|Default|GetLast)))
            (CallFunction|OnChatModelResponse (.RightS (Utilities|String|Split _returnvalue (Variables|Default|GetLast))))
            (Variables|Default|SetLast _returnvalue)))
        (:CompletedDelegate
          (CallFunction|OnChatModelCompleted))
        (:CancelDelegate
          (CallFunction|OnChatModelCancel))
        (:ErrorDelegate
          (CallFunction|OnChatModelError _message))))))

(event Custom|StopChatModel
  (Variables|Default|SetIsRuning false)
  (CallFunction|ClearCache)
  (bind _request_task (Variables|Default|GetRequest%20Task)
    (:then
      (Class|DifyModelAsyncTaskAction|CancelDifyModelAsyncTaskAction _request_task))
    (:else)))

(event Custom|ClearCache
  (Variables|Default|SetTempQuestion "")
  (Variables|Default|SetConversationID "")
  (Variables|Default|SetTemp "")
  (Variables|Default|SetLast "")
  (Variables|Default|Set总的字符串 "")
  (Variables|Default|Set已合成语音字符串 ""))

(event Custom|OnChatModelCancel
  (CallFunction|StopChatModel))

(event Custom|OnChatModelResponse
  (params (Result :type String))
  (Development|PrintString (Utilities|String|Append "[语音大模型]：原生输出：" Result))
  (Variables|Default|Set总的字符串 (Utilities|String|Append (Variables|Default|Get总的字符串) Result))
  (if (<= (Utilities|String|Len (.RightS (Utilities|String|Split (Variables|Default|Get总的字符串) (Variables|Default|Get已合成语音字符串)))) 200)
    (if (CallFunction|分句条件判断 (.RightS (Utilities|String|Split (Variables|Default|Get总的字符串) (Variables|Default|Get已合成语音字符串))) 30)
      (Default|CallChatModelGeneratedDelegate (.RightS (Utilities|String|Split (Variables|Default|Get总的字符串) (Variables|Default|Get已合成语音字符串))))
      (Variables|Default|Set已合成语音字符串 (Utilities|String|Append (Variables|Default|Get已合成语音字符串) (.RightS (Utilities|String|Split (Variables|Default|Get总的字符串) (Variables|Default|Get已合成语音字符串))))))))

(event Custom|OnChatModelCompleted
  (bind _总的字符串 (Variables|Default|Get总的字符串))
  (bind _已合成语音字符串 (Variables|Default|Get已合成语音字符串))
  (bind (_lefts _rights _returnvalue) (Utilities|String|Split _总的字符串 _已合成语音字符串))
  (Utilities|FlowControl|Sequence
    (:then_0
      (if (Utilities|Array|IsEmpty (Variables|Default|Get总的字符串))
        (CallFunction|OnChatModelError "[大模型]：总的输出为空，再执行一次")
        (CallFunction|StartChatModel (Variables|Default|GetTempQuestion) (Variables|Default|GetTempType))
        (elif (Utilities|Enum|NotEqual(Enum) (Variables|Default|Get总的字符串) (Variables|Default|Get已合成语音字符串))
          (if _returnvalue
            (if (<= (Utilities|String|Len _rights) 200)
              (Default|CallChatModelGeneratedDelegate _rights)
              (else
                (bind _returnvalue_2 (Class|ChatModelsSubsystem|GetSpecialSplitStrings (Subsystems|GetChatModelsSubsystem) _rights "。" 30))
                (for _array_element _returnvalue_2
                  (Default|CallChatModelGeneratedDelegate _array_element))))))))
    (:then_1
      (Variables|Default|SetIsRuning false)
      (Default|CallChatModelCompletedDelegate))))

(event Custom|OnChatModelError
  (params (Reason :type String))
  (Default|CallChatModelErrorDelegate Reason))

(fn 分句条件判断
  (params (SourceString :type String) (MinLength :type Integer))
  (return (and (> (Utilities|String|Len SourceString) MinLength) (Math|Boolean|ORBoolean (Utilities|String|EndsWith SourceString "。") (Utilities|String|EndsWith SourceString "，") (Utilities|String|EndsWith SourceString "！") (Utilities|String|EndsWith SourceString "：") (Utilities|String|EndsWith SourceString "!") (Utilities|String|EndsWith SourceString "、") (Utilities|String|EndsWith SourceString "；") (Utilities|String|Contains SourceString ". " false true) (Utilities|String|Contains SourceString ", " false true)))))