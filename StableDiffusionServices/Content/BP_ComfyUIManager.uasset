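; BP_ComfyUIManager runs Stable Diffusion text-to-image jobs on ComfyUI and hands back the generated textures.
; A WebSocket listener relays queue, start, execution, progress and completion events through dispatchers.
; Macros wrap async HTTP submit, query and result calls; image retrieval chains query into download, then broadcasts the texture.
; An IsRunning flag blocks overlapping submissions until retrieval, failure or cancellation, and stored task handles allow cancelling requests.
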(event Custom|提交文生图任务
  (params (InPrompt :type String))
  (if (Variables|Default|GetIsRunning)
    (Development|PrintString "[SDComfyUI]:前一个任务未完成Warning")
    (else
      (Variables|Default|SetIsRunning true)
      (bind (_submitttitask _prompt_id) (Utilities|提交文生图任务 InPrompt 20)
        (:then
          (Variables|Default|SetHTTP%20Submit%20Task%20Request%20Task _submitttitask))
        (:Completed
          (Variables|Default|SetPrompt%20ID _prompt_id))
        (:Cancel
          (Variables|Default|SetIsRunning false :!label _label))
        (:Error
          (goto _label))))))

(event Custom|查询文生图任务状态
  (params (PromptID :type String))
  (bind (_findttitask _image_file_name _type) (Utilities|查询文生图任务状态 PromptID 20)
    (:then
      (Variables|Default|SetHTTP%20Get%20Task%20Info%20Request%20Task _findttitask))
    (:Completed
      (Variables|Default|SetImage%20File%20Name _image_file_name)
      (Variables|Default|SetImage%20Type _type))
    (:Cancel
      (Variables|Default|SetIsRunning false :!label _label))
    (:Error
      (goto _label))))

(event Custom|获取文生图任务结果
  (bind (_resultttitask _texture_2ddynamic) (Utilities|获取文生图任务结果 (Variables|Default|GetImage%20File%20Name) (Variables|Default|GetImage%20Type) 20)
    (:then
      (Variables|Default|SetHTTP%20Get%20Task%20Result%20Request%20Task _resultttitask))
    (:Completed
      (Variables|Default|SetTexture%202DDynamic _texture_2ddynamic))
    (:Cancel
      (Variables|Default|SetIsRunning false :!label _label))
    (:Error
      (goto _label))))

(event Custom|获取文生图任务图片
  (params (PromptID :type String))
  (bind (_findttitask _image_file_name _type) (Utilities|查询文生图任务状态 PromptID 20)
    (:then
      (Variables|Default|SetHTTP%20Get%20Task%20Info%20Request%20Task _findttitask))
    (:Completed
      (bind (_resultttitask _texture_2ddynamic) (Utilities|获取文生图任务结果 _image_file_name _type 20)
        (:then
          (Variables|Default|SetHTTP%20Get%20Task%20Result%20Request%20Task _resultttitask))
        (:Completed
          (Utilities|IsValid _texture_2ddynamic
            (:Is%20Valid
              (Default|CallTTIImageGotDispatcher _texture_2ddynamic))
            (:Is%20Not%20Valid
              _))
          (Variables|Default|SetIsRunning false :!label _label))
        (:Cancel
          (goto _label))
        (:Error
          (goto _label))))
    (:Cancel
      (goto _label))
    (:Error
      (goto _label))))

(event Custom|停止文生图任务
  (Utilities|FlowControl|Sequence
    (:then_0
      (bind _http_submit_task_request_task (Variables|Default|GetHTTP%20Submit%20Task%20Request%20Task)
        (:then
          (Class|ComfyUISubmitTaskAsyncAction|Cancel _http_submit_task_request_task))
        (:else)))
    (:then_1
      (bind _http_get_task_info_request_task (Variables|Default|GetHTTP%20Get%20Task%20Info%20Request%20Task)
        (:then
          (Class|ComfyUIGetTaskInfoAsyncAction|Cancel _http_get_task_info_request_task))
        (:else)))
    (:then_2
      (bind _http_get_task_result_request_task (Variables|Default|GetHTTP%20Get%20Task%20Result%20Request%20Task)
        (:then
          (Class|ComfyUIGetTaskResultAsyncAction|Cancel _http_get_task_result_request_task))
        (:else)))
    (:then_3
      (Variables|Default|SetIsRunning false))))

(event Custom|停止全局监听事件
  (bind _web_socket_task_listen_task (Variables|Default|GetWeb%20Socket%20Task%20Listen%20Task)
    (:then
      (Class|ComfyUIListenAsyncAction|Cancel _web_socket_task_listen_task))
    (:else)))

(event Custom|开启全局监听事件
  (bind (_asynctaskproxy _output) (|Connect)
    (:then
      (Variables|Default|SetWeb%20Socket%20Task%20Listen%20Task _asynctaskproxy))
    (:ProcessDelegate
      (bind _asstable_diffusion_listen_output (Utilities|Casting|CastToStableDiffusionListenOutput _output))
      (switch Utilities|FlowControl|Switch|SwitchonListenType (Variables|/Script/StableDiffusionServices.StableDiffusionListenOutput|GetType _asstable_diffusion_listen_output)
        (:Status
          (Development|PrintString (Utilities|String|Append "[SDComfyUI全局状态]：queue_remaining：" (Utilities|String|ToString(Integer) (Variables|/Script/StableDiffusionServices.StableDiffusionListenOutput|GetQueueRemaining _asstable_diffusion_listen_output))))
          (Default|CallGListenQueueChangedDispatcher (Variables|/Script/StableDiffusionServices.StableDiffusionListenOutput|GetQueueRemaining _asstable_diffusion_listen_output)))
        (:ExecutionStart
          (Development|PrintString (Utilities|String|Append "[SDComfyUI全局状态]：开始执行任务，prompt_id：" (Variables|/Script/StableDiffusionServices.StableDiffusionListenOutput|GetPromptID _asstable_diffusion_listen_output)))
          (Default|CallGListenTaskStartDispatcher (Variables|/Script/StableDiffusionServices.StableDiffusionListenOutput|GetPromptID _asstable_diffusion_listen_output)))
        (:Executing
          (Development|PrintString (Utilities|String|Append "[SDComfyUI全局状态]：正在执行任务，node：" (Variables|/Script/StableDiffusionServices.StableDiffusionListenOutput|GetNode _asstable_diffusion_listen_output) "，prompt_id：" (Variables|/Script/StableDiffusionServices.StableDiffusionListenOutput|GetPromptID _asstable_diffusion_listen_output)))
          (Default|CallGListenTaskExcutingDispatcher))
        (:Progress
          (Development|PrintString (Utilities|String|Append "[SDComfyUI全局状态]：任务进度：" (Utilities|String|ToString(Float) (* (/ (Math|Conversions|ToFloat(Integer) (Variables|/Script/StableDiffusionServices.StableDiffusionListenOutput|GetValue _asstable_diffusion_listen_output)) (Math|Conversions|ToFloat(Integer) (Variables|/Script/StableDiffusionServices.StableDiffusionListenOutput|GetMax _asstable_diffusion_listen_output))) 1e+02)) "%"))
          (Default|CallGListenTaskProgressDispatcher (/ (Math|Conversions|ToFloat(Integer) (Variables|/Script/StableDiffusionServices.StableDiffusionListenOutput|GetValue _asstable_diffusion_listen_output)) (Math|Conversions|ToFloat(Integer) (Variables|/Script/StableDiffusionServices.StableDiffusionListenOutput|GetMax _asstable_diffusion_listen_output)))))
        (:Completed
          (Development|PrintString (Utilities|String|Append "[SDComfyUI全局状态]：执行任务结束，prompt_id：" (Variables|/Script/StableDiffusionServices.StableDiffusionListenOutput|GetPromptID _asstable_diffusion_listen_output)))
          (Default|CallGListenTaskCompletedDispatcher (Variables|/Script/StableDiffusionServices.StableDiffusionListenOutput|GetPromptID _asstable_diffusion_listen_output)))))
    (:CompletedDelegate
      (Development|PrintString "[SDComfyUI]:监听停止工作Error" :!label _label))
    (:CancelDelegate
      (goto _label))
    (:ErrorDelegate
      (goto _label))))

(fn ConstructionScript)

(fn 获取ComfyUIClientID
  (return (Class|StableDiffusionServicesSubsystem|GetComfyUIClientID (Subsystems|GetStableDiffusionServicesSubsystem))))