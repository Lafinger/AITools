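; Text-to-image controller Blueprint that generates images through ComfyUI from prompts entered in a WBP_SDExample widget.
; On init it creates the widget, binds its generate and stop buttons, and starts ComfyUIManager's global listener.
; Generate sends the prompt through XunFei translation, then submits the result as a ComfyUI task.
; Manager callbacks update the progress bar, fetch the completed image and display it, while stop and exit events cancel translation and generation.
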(event Custom|初始化文生图
  (bind _returnvalue (Game|GetPlayerController 0))
  (bind _comfyuimanager (Variables|Default|GetComfyUIManager))
  (Utilities|FlowControl|Sequence
    (:then_0
      (bind _returnvalue_2 (UserInterface|CreateWidget "/StableDiffusionServices/WBP_SDExample.WBP_SDExample_C" _returnvalue))
      (bind _output_get (Variables|Default|SetSDWidget _returnvalue_2))
      (UserInterface|Viewport|AddtoViewport _output_get 0)
      (Variables|/Script/Engine.PlayerController|SetbShowMouseCursor _returnvalue true)
      (EventDispatchers|BindEventtoGenerateBtnClickDispatcher (Variables|Default|GetSDWidget) (delegate Custom|触发开始生成图片按钮的回调))
      (EventDispatchers|BindEventtoStopBtnClickDispatcher (Variables|Default|GetSDWidget) (delegate Custom|触发停止生成图片按钮的回调)))
    (:then_2
      (Default|开启全局监听事件 _comfyuimanager)
      (EventDispatchers|BindEventtoGListenTaskCompletedDispatcher _comfyuimanager (delegate Custom|文胜图任务完成回调))
      (EventDispatchers|AssignGListenTaskProgressDispatcher _comfyuimanager (delegate Custom|文胜图任务进度回调))
      (EventDispatchers|BindEventtoTTIImageGotDispatcher _comfyuimanager (delegate Custom|获取文生图图片完成的回调)))))

(event Custom|退出音生图
  (Utilities|FlowControl|Sequence
    (:then_0
      (CallFunction|停止文生图))
    (:then_1
      (Default|停止全局监听事件 (Variables|Default|GetComfyUIManager)))))

(event Custom|开始文生图
  (params (SourceText :type String))
  (Class|IVXunFeiSpeechFunctionLibrary|XunFeiBeginTranslate SourceText (Utilities|Struct|MakeXunFeiTranslateOptions 3 "" "cn" "en") (delegate Custom|生成按钮点击后翻译)))

(event Custom|文胜图任务完成回调
  (params (PromptID :type String))
  (Default|获取文生图任务图片 (Variables|Default|GetComfyUIManager) PromptID))

(event Custom|触发停止生成图片按钮的回调
  (CallFunction|停止文生图))

(event Custom|文胜图任务进度回调
  (params (Progress :type Float%20%28double-precision%29))
  (Default|SetProgressBarPercent (Variables|Default|GetSDWidget) Progress))

(event Custom|触发开始生成图片按钮的回调
  (CallFunction|开始文生图 (Default|GetPromptText (Variables|Default|GetSDWidget))))

(event Custom|停止文生图
  (Utilities|FlowControl|Sequence
    (:then_0
      (Class|IVXunFeiSpeechFunctionLibrary|XunFeiStopTranslate))
    (:then_1
      (Default|停止文生图任务 (Variables|Default|GetComfyUIManager)))))

(event Custom|退出文生图
  (Utilities|FlowControl|Sequence
    (:then_0
      (CallFunction|停止文生图))
    (:then_1
      (Default|停止全局监听事件 (Variables|Default|GetComfyUIManager)))))

(event Custom|获取文生图图片完成的回调
  (params (Texture2DDynamic :type Texture%202D%20Dynamic%20Object%20Reference))
  (Default|SetComfyUISDImage (Variables|Default|GetSDWidget) Texture2DDynamic))

(event Custom|生成按钮点击后翻译
  (params (bIsSuccess :type Boolean) (FinalResult :type String))
  (if bIsSuccess
    (Default|提交文生图任务 (Variables|Default|GetComfyUIManager) FinalResult)
    (Default|SetTranslatedText (Variables|Default|GetSDWidget) FinalResult)
    (else
      (Development|PrintString "[翻译]：翻译失败"))))

(fn ConstructionScript)