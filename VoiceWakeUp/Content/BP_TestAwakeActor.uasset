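; Test actor that exercises the VoiceWakeUpSubsystem through custom events for initializing, starting, stopping and exiting voice wake-up.
; Initialization calls MsgLogin and, only on success, binds handlers to the trigger, completed and failed delegates.
; Each handler prints a Chinese status message, with the error code appended on failure.
; Exit stops the subsystem, logs out and unbinds all three delegates.
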(event Custom|停止语音唤醒
  (Class|VoiceWakeUpSubsystem|Stop (|VoiceWakeUpSubsystem)))

(event Custom|开始语音唤醒
  (Class|VoiceWakeUpSubsystem|Start (|VoiceWakeUpSubsystem)))

(event Custom|初始化语音唤醒
  (bind _returnvalue (|VoiceWakeUpSubsystem))
  (bind _returnvalue_2 (Class|VoiceWakeUpSubsystem|MsgLogin _returnvalue))
  (if _returnvalue_2
    (EventDispatchers|AssignWakeUpTriggerDelegate _returnvalue (delegate Custom|WakeUpTriggerDelegate_Event))
    (EventDispatchers|AssignWakeUpCompletedDelegate _returnvalue (delegate Custom|WakeUpCompletedDelegate_Event))
    (EventDispatchers|AssignWakeUpFailedDelegate _returnvalue (delegate Custom|WakeUpFailedDelegate_Event))))

(event Custom|WakeUpTriggerDelegate_Event
  (Development|PrintString "[语音唤醒]：触发唤醒"))

(event Custom|WakeUpCompletedDelegate_Event
  (Development|PrintString "[语音唤醒]：唤醒完成"))

(event Custom|WakeUpFailedDelegate_Event
  (params (ErrorCode :type Integer))
  (Development|PrintString (Utilities|String|Append "[语音唤醒]：唤醒出错， 错误码：" (Utilities|String|ToString(Integer) ErrorCode))))

(event Custom|退出语音唤醒
  (bind _returnvalue (|VoiceWakeUpSubsystem))
  (Class|VoiceWakeUpSubsystem|Stop _returnvalue)
  (Class|VoiceWakeUpSubsystem|MsgLogout _returnvalue)
  (EventDispatchers|UnbindallEventsfromWakeUpTriggerDelegate _returnvalue)
  (EventDispatchers|UnbindallEventsfromWakeUpCompletedDelegate _returnvalue)
  (EventDispatchers|UnbindallEventsfromWakeUpFailedDelegate _returnvalue))

(fn ConstructionScript)