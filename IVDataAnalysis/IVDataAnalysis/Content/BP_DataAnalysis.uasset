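; Test actor that imports a question-and-answer spreadsheet at runtime and prints it for checking.
; Pressing 2 loads an Excel workbook from the project directory, reads Sheet1 into a runtime-created DataTable (题目/答案 struct), then prints each row's answer.
; Unconnected leftover chains try CSV import from a hardcoded absolute path, printing questions, and JSON-string import.
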(event EventBeginPlay)

(event Collision|EventActorBeginOverlap
  (params (OtherActor :type Actor%20Object%20Reference)))

(event EventTick
  (params (DeltaSeconds :type Float%20%28single-precision%29)))

(event Input|KeyboardEvents|2
  (params (Key :type Key%20Structure :default "None"))
  (:Pressed
    (bind _returnvalue (Class|IVExcelWorkBook|LoadWorkBookfromFile (Utilities|String|Append (Class|IVisualFileHeplerBPLibrary|GetProjectDir) "100题.xlsx")))
    (bind _returnvalue_2 (Class|IVRuntimeDataTableLibrary|CreateRunTimeTable (Utilities|Struct|MakeS_AN) "ID" true true))
    (bind _output_get (Variables|Default|SetTestTable _returnvalue_2))
    (bind _returnvalue_3 (Class|IVExcelWorkBook|GetSheetwithTitle _returnvalue _output_get "Sheet1"))
    (if _returnvalue_3
      (bind _outrownames (Class|IVRuntimeDataTableLibrary|GetTableRowNames (Variables|Default|GetTestTable)))
      (for _array_element _outrownames
        (bind _row (Class|IVRuntimeDataTableLibrary|GetRowfromTable (Variables|Default|GetTestTable) _array_element))
        (Development|PrintString (.答案 (Utilities|Struct|BreakS_AN _row)))))))

(fn ConstructionScript)