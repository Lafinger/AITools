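; Test actor that wraps the VoiceSynthesisSubsystem to run iFlytek (XunFei) text-to-speech.
; Events bind and unbind queue delegates, start and stop the queue, enqueue text tasks with a fixed voice preset, and allow stopping once the queue empties.
; Completed tasks pass valid SoundWaves to a dispatcher, with print-string logging throughout.
; A separate event synthesizes text straight to a WAV file, bypassing the queue.
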(event Custom|初始化语音合成
  (bind _returnvalue (|VoiceSynthesisSubsystem))
  (EventDispatchers|AssignQueueWorkingStartDelegate _returnvalue (delegate Custom|语音合成初始化完成的回调))
  (EventDispatchers|AssignTaskCompletedDelegate _returnvalue (delegate Custom|语音合成一个完成的回调))
  (EventDispatchers|AssignQueueWorkingCompletedDelegate _returnvalue (delegate Custom|语音合成所有任务完成的回调))
  (EventDispatchers|AssignTaskErrorDelegate _returnvalue (delegate Custom|语音合成一个出错的回调)))

(event Custom|退出语音合成
  (bind _returnvalue (|VoiceSynthesisSubsystem))
  (EventDispatchers|UnbindallEventsfromQueueWorkingStartDelegate _returnvalue)
  (EventDispatchers|UnbindallEventsfromTaskCompletedDelegate _returnvalue)
  (EventDispatchers|UnbindallEventsfromQueueWorkingCompletedDelegate _returnvalue)
  (EventDispatchers|UnbindallEventsfromTaskErrorDelegate _returnvalue))

(event Custom|合成语音文件
  (params (SourceText :type String) (FilePath :type String))
  (if (and (not (Utilities|Array|IsEmpty SourceText)) (not (Utilities|Array|IsEmpty FilePath)))
    (|XunFeiTexttoWavFile SourceText (Utilities|Struct|MakeXunFeiTTSOptions "x4_mengmengneutral" 50) FilePath
      (:OnConnectionError
        (Development|PrintString (Utilities|String|ToString(Text) (Utilities|Text|FormatText "[工具]：合成语音文件{0}Error，文本为：{1}！" FilePath SourceText))))
      (:OnClose
        (Development|PrintString (Utilities|String|ToString(Text) (Utilities|Text|FormatText "[工具]：合成语音文件{0}完成，文本为：{1}" FilePath SourceText)))))
    (else
      (Development|PrintString "[工具]：需要合成的文本或路径为空 Error!"))))

(event Custom|语音合成初始化完成的回调
  (Development|PrintString "[语音合成]：初始化完成"))

(event Custom|语音合成一个完成的回调
  (params (VoiceText :type String) (SourceText :type String) (FileAbsolutePath :type String) (SoundWave :type Sound%20Wave%20Object%20Reference))
  (Utilities|IsValid SoundWave
    (:Is%20Valid
      (Development|PrintString (Utilities|String|Append "[语音合成]：成功，合成内容为：" VoiceText))
      (Default|CallSoundWaveSynthesisCompletedDispatcher SoundWave))))

(event Custom|语音合成一个出错的回调
  (params (ErrorMessage :type String))
  (Development|PrintString (Utilities|String|Append "[语音合成]：出错：" ErrorMessage)))

(event Custom|开始语音合成
  (Development|PrintString "[语音合成]：开始")
  (Class|VoiceSynthesisSubsystem|StartQueueWorking (|VoiceSynthesisSubsystem) false))

(event Custom|添加语音合成任务
  (params (InText :type String))
  (Development|PrintString (Utilities|String|Append "[语音合成]：添加语音合成任务文本为：" InText))
  (Class|VoiceSynthesisSubsystem|EnqueueVoiceSynthesisTask (|VoiceSynthesisSubsystem) InText InText (Utilities|Struct|MakeXunFeiTTSOptions "x4_mengmengneutral" 50)))

(event Custom|停止语音合成
  (Development|PrintString "[语音合成]：停止")
  (Class|VoiceSynthesisSubsystem|StopQueueWorking (|VoiceSynthesisSubsystem)))

(event Custom|当所有语音合成任务完成时可以停止队列工作
  (Development|PrintString "[语音合成]：可以停止工作")
  (Class|VoiceSynthesisSubsystem|CanQueueCompletedWhileQueueEmpty (|VoiceSynthesisSubsystem)))

(event Custom|语音合成所有任务完成的回调
  (Development|PrintString "[语音合成]：所有语音合成结束"))

(fn ConstructionScript)